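; Player controller for SupplyCo that owns the player's inventory and resource stats: gold, reputation, debt and fingers.
; On BeginPlay it enables mouse click and hover events, spawns BP_Inventory, then fills it from the first DT_ItemCards rows through BP_CommandAddItem command objects.
; Setter functions store each stat and broadcast changes through dispatchers, with zero gold flagging the player as broke.
; The E key broadcasts a debug event.
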(event `self.ReceiveBeginPlay`
  (`self.StartMouseEvents`)
  (`self.Listen For Debug`)
  (bind _returnvalue (`|SpawnActorFromClass` "/Game/SupplyCo/Blueprints/BP_Inventory.BP_Inventory_C" (`KismetMathLibrary.MakeTransform` (0.0 0.0 0.0)) "Undefined" "OverrideRootScale" null null))
  (bind _output_get (set `self.Inventory` _returnvalue))
  (`self.OnInventoryCreated` _output_get)
  (`self.GenerateStartingItems`))

(event `GenerateStartingItems`
  ;[1 1 1] Add starting Items to Inventory
  (for _index (range (+ (`self.StartingInventory`) 1))
    (bind _outrownames (`DataTableFunctionLibrary.GetDataTableRowNames` "/Game/SupplyCo/Blueprints/DT_ItemCards.DT_ItemCards"))
    (bind _returnvalue (`|GetDataTableRow` "/Game/SupplyCo/Blueprints/DT_ItemCards.DT_ItemCards" (`|GetArrayItem` _outrownames _index))
      (:`then`
        (bind _returnvalue_2 (`|GenericCreateObject` "/Game/SupplyCo/Blueprints/BP_CommandAddItem.BP_CommandAddItem_C" self _returnvalue))
        (`/Game/SupplyCo/Blueprints/BP_Command.Execute` _returnvalue_2 self)))))

(event `Listen For Debug`
  (`self.EnableInput` self))

(event `Key|E`
  (params (Key :type "Key Structure"))
  (:`Pressed`
    (`self.OnDebugKeyPressed`)))

(event `StartMouseEvents`
  (set `self.bEnableMouseOverEvents` true)
  (set `self.bEnableClickEvents` true))

(fn `ChangeDebt`
  (params (NewDebt :type Integer))
  (bind _output_get (set `self.Debt` NewDebt))
  (`self.OnDebtChanged` _output_get))

(fn `ChangeFingers`
  (params (NewFingers :type Integer))
  (bind _output_get (set `self.Fingers` NewFingers))
  (`self.OnFingersChanged` _output_get))

(fn `ChangeMoney`
  (params (NewMoney :type Integer))
  (bind _output_get (set `self.Gold` NewMoney))
  (if (== _output_get 0)
    (set `self.IsBroke` true)
    (else
      (set `self.IsBroke` false)))
  (`self.OnMoneyChanged` _output_get (`self.IsBroke`)))

(fn `ChangeReputation`
  (params (Reputation :type Integer))
  (bind _output_get (set `self.Reputation` Reputation))
  (`self.OnReputationChanged` _output_get))

(fn `UserConstructionScript`)