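; Event variant of a customer actor that presents an event in a speech bubble and ignores clicks on itself.
; StartInteraction spawns a bubble actor hosting an event widget, then places it at the game mode's current speech bubble location with a slight Z offset.
; The OnBubbleCreated dispatcher binds the widget's OnEventDealtWith, which destroys the bubble and signals that the customer is handled.
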(event `self.Handle Click`
  ;[1 1 1] Do nothing, it's an event
)

(event `self.ReceiveBeginPlay`
  (`parent.ReceiveBeginPlay`)
  (add `self.OnBubbleCreated` (delegate `Bubble Created`)))

(event `Bubble Created`
  (bind _aswbp_event_bubble (cast `/Game/SupplyCo/Blueprints/WBP_EventBubble` (`/Game/SupplyCo/Blueprints/BP_Bubble.UserWidget` (`self.EventBubble`))))
  (add `/Game/SupplyCo/Blueprints/WBP_EventBubble.OnEventDealtWith` _aswbp_event_bubble (delegate `Deal With Customer`)))

(event `Deal With Customer`
  (`self.K2_DestroyActor` (`self.EventBubble`))
  (`self.CustomerHandled`))

(fn `CreateEventBubble`
  (params (Event :type "/Game/SupplyCo/Blueprints/BP_Event Object Reference"))
  (returns (EventBubble :type "/Game/SupplyCo/Blueprints/BP_EventBubbleActor Object Reference"))
  (bind _returnvalue (`|CreateWidget` "/Game/SupplyCo/Blueprints/WBP_EventBubble.WBP_EventBubble_C" (cast `/Game/SupplyCo/Blueprints/BP_PlayerController` (`GameplayStatics.GetPlayerController` 0) :!pure true) Event))
  (bind _returnvalue_2 (`|SpawnActorFromClass` "/Game/SupplyCo/Blueprints/BP_EventBubbleActor.BP_EventBubbleActor_C" (`KismetMathLibrary.MakeTransform` (0.0 0.0 0.0)) "Undefined" "OverrideRootScale" null _returnvalue null))
  (return _returnvalue_2))

(fn `StartInteraction`
  (bind (_returnvalue_x _returnvalue_y _returnvalue_z) (`KismetMathLibrary.BreakVector` (`self.K2_GetActorLocation` (`/Game/SupplyCo/Blueprints/BP_Gamemode.CurrentSpeechBubble` (cast `/Game/SupplyCo/Blueprints/BP_Gamemode` (`GameplayStatics.GetGameMode`) :!pure true)))))
  (bind _eventbubble (`self.CreateEventBubble` (`self.Event`)))
  (bind _output_get (set `self.EventBubble` _eventbubble))
  (`self.OnBubbleCreated`)
  (`self.K2_SetActorLocation` _output_get (`KismetMathLibrary.MakeVector` _returnvalue_x _returnvalue_y _returnvalue_z) false false)
  (`self.K2_AddActorLocalOffset` _eventbubble (0.0 0.0 2.0) false false))

(fn `UserConstructionScript`)