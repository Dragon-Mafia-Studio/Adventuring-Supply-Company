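; BP_CustomerActorSelling is a customer actor, named for selling, whose interaction switches the game mode into a specific state.
; On BeginPlay it binds to the player controller's inventory-created event, then subscribes to that inventory's item-removed event.
; When an item is removed while the game mode is in that same state, it calls CustomerHandled.
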(event `self.ReceiveBeginPlay`
  (`parent.ReceiveBeginPlay`)
  (add `/Game/SupplyCo/Blueprints/BP_PlayerController.OnInventoryCreated` (cast `/Game/SupplyCo/Blueprints/BP_PlayerController` (`GameplayStatics.GetPlayerController` 0) :!pure true) (delegate `OnInventoryCreated`)))

(event `OnInventoryCreated`
  (params (Inventory :type "/Game/SupplyCo/Blueprints/BP_Inventory Object Reference"))
  (add `/Game/SupplyCo/Blueprints/BP_Inventory.OnItemRemoved` Inventory (delegate `HandleCustomer`)))

(event `HandleCustomer`
  (params (ItemRemoved :type "/Game/SupplyCo/Blueprints/F_ItemData Structure") (Inventory :type "/Game/SupplyCo/Blueprints/BP_Inventory Object Reference"))
  (if (`|EnumEquality` (`/Game/SupplyCo/Blueprints/BP_Gamemode.State` (cast `/Game/SupplyCo/Blueprints/BP_Gamemode` (`GameplayStatics.GetGameMode`) :!pure true)) "NewEnumerator2")
    (`self.CustomerHandled`)))

(fn `StartInteraction`
  (`/Game/SupplyCo/Blueprints/BP_Gamemode.ChangeState` (cast `/Game/SupplyCo/Blueprints/BP_Gamemode` (`GameplayStatics.GetGameMode`) :!pure true) "NewEnumerator2"))

(fn `UserConstructionScript`)