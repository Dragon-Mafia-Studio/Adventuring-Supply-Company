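; Clickable shop item actor that shows its item's sprite and lets the player sell or buy it.
; Cursor hover spawns a single item info box at the hit location, removed when hover ends.
; Clicks branch on gamemode state: selling clears the shelf slot, while buying checks gold and space, showing errors on failure.
; Gold and inventory changes run through command objects, and successful trades notify the current customer.
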(event `self.ReceiveBeginPlay`
  ;[1 1 1] Set the sprite for the item
  (`PaperSpriteComponent.SetSprite` (`self.PaperSprite`) (`.Picture_20_C0DE07CD432E5F2C2EA17BBF52B3D54A` (break `/Game/SupplyCo/Blueprints/F_ItemData` (`self.Item`)))))

(event `self.ClickListener.OnBeginCursorOver`
  (params (TouchedComponent :type "PrimitiveComponent Object Reference"))
  (bind _hitresult (`PlayerController.GetHitResultUnderCursorByChannel` (cast `/Game/SupplyCo/Blueprints/BP_PlayerController` (`GameplayStatics.GetPlayerController` 0) :!pure true) "TraceTypeQuery1" true))
  ;[1 1 1] Create/Destroy the item info box
  (`/Engine/EditorBlueprintResources/StandardMacros.DoOnce` false :!label _label
    (:`Completed`
      (bind _returnvalue (`|SpawnActorFromClass` "/Game/SupplyCo/Blueprints/BP_ItemInfo.BP_ItemInfo_C" (`KismetMathLibrary.MakeTransform` (`KismetMathLibrary.MakeVector` (.x (`.Location` (`GameplayStatics.BreakHitResult` _hitresult))) (.y (`.Location` (`GameplayStatics.BreakHitResult` _hitresult))) 35.0)) "Undefined" "OverrideRootScale" null (`self.Item`) null))
      (bind _output_get (set `self.ItemInfo` _returnvalue))
      (`self.K2_AddActorLocalOffset` _output_get (50.0 200.0 0.0) false false))))

(event `self.ClickListener.OnEndCursorOver`
  (params (TouchedComponent :type "PrimitiveComponent Object Reference"))
  ;[1 1 1] Create/Destroy the item info box
  (bind _iteminfo (`self.ItemInfo`)
    (:`then`
      (`self.K2_DestroyActor` _iteminfo)
      (goto _label :!via `Reset`))
    (:`else`
      (goto _label :!via `Reset`))))

(event `self.ClickListener.OnClicked`
  (params (TouchedComponent :type "PrimitiveComponent Object Reference") (ButtonPressed :type "Key Structure"))
  (bind _asbp_player_controller (cast `/Game/SupplyCo/Blueprints/BP_PlayerController` (`GameplayStatics.GetPlayerController` 0) :!pure true))
  (bind _asbp_player_controller_2 (cast `/Game/SupplyCo/Blueprints/BP_PlayerController` (`GameplayStatics.GetPlayerController` 0) :!pure true))
  (bind _errorbox (`/Game/SupplyCo/Blueprints/BP_Gamemode.ErrorBox` (cast `/Game/SupplyCo/Blueprints/BP_Gamemode` (`GameplayStatics.GetGameMode`) :!pure true)))
  (bind _errorbox_2 (`/Game/SupplyCo/Blueprints/BP_Gamemode.ErrorBox` (cast `/Game/SupplyCo/Blueprints/BP_Gamemode` (`GameplayStatics.GetGameMode`) :!pure true)))
  ;[1 1 1] Check game state
  (switch `/Game/SupplyCo/Blueprints/EGameState` (`/Game/SupplyCo/Blueprints/BP_Gamemode.State` (cast `/Game/SupplyCo/Blueprints/BP_Gamemode` (`GameplayStatics.GetGameMode`) :!pure true))
    (:`NewEnumerator2`
      ;[1 1 1] If you click on an item while in selling mode
      (bind _returnvalue (`|GenericCreateObject` "/Game/SupplyCo/Blueprints/BP_CommandChangeGold.BP_CommandChangeGold_C" self (`.Price_11_87D75CD5441D943E04940E99A4C19D17` (break `/Game/SupplyCo/Blueprints/F_ItemData` (`self.Item`)))))
      (`/Game/SupplyCo/Blueprints/BP_Command.Execute` _returnvalue _asbp_player_controller)
      (bind _returnvalue_2 (`|GenericCreateObject` "/Game/SupplyCo/Blueprints/BP_CommandRemoveItem.BP_CommandRemoveItem_C" self (`self.Item`)))
      (`/Game/SupplyCo/Blueprints/BP_Command.Execute` _returnvalue_2 _asbp_player_controller)
      (bind _asbp_shelf_slot (cast `/Game/SupplyCo/Blueprints/BP_ShelfSlot` (`self.GetAttachParentActor` self))
        (:`then`
          (`/Game/SupplyCo/Blueprints/BP_ShelfSlot.RemoveItemFromSlot` _asbp_shelf_slot self)
          (`self.K2_DestroyActor` (`self.ItemInfo`))
          (`GameplayStatics.PlaySound2D` "/Game/SupplyCo/Assets/Sounds/A_CashRegister.A_CashRegister" 1.0 1.0 0.0 null null)
          (`/Game/SupplyCo/Blueprints/BP_CustomerActor.CustomerHandled` (`/Game/SupplyCo/Blueprints/BP_Gamemode.CurrentCustomer` (cast `/Game/SupplyCo/Blueprints/BP_Gamemode` (`GameplayStatics.GetGameMode`) :!pure true))))
        (:`CastFailed`
          (`KismetSystemLibrary.PrintString` "ERROR. ITEM NOT ATTACHED TO SHELF SLOT"))))
    (:`NewEnumerator3`
      (if (not (`self.IsInInventory`))
        ;[1 1 1] Do you have enough money
        (if (or (`/Game/SupplyCo/Blueprints/BP_PlayerController.IsBroke` _asbp_player_controller_2) (< (+ (`/Game/SupplyCo/Blueprints/BP_PlayerController.Gold` _asbp_player_controller_2) (* (`.Price_11_87D75CD5441D943E04940E99A4C19D17` (break `/Game/SupplyCo/Blueprints/F_ItemData` (`self.Item`))) -1)) 0))
          (`/Game/SupplyCo/Blueprints/WBP_ErrorDialogue.SetErrorText` _errorbox_2 "You don't have enough money!")
          (`/Game/SupplyCo/Blueprints/WBP_ErrorDialogue.SetBoxVisibility` _errorbox_2 true)
          (else
            ;[1 1 1] If you click on an item in buying mode
            (bind _returnvalue_3 (`|GenericCreateObject` "/Game/SupplyCo/Blueprints/BP_CommandAddItem.BP_CommandAddItem_C" self (`self.Item`)))
            (bind _issuccessful (`/Game/SupplyCo/Blueprints/BP_Command.Execute` _returnvalue_3 _asbp_player_controller))
            (if _issuccessful
              (bind _returnvalue_4 (`|GenericCreateObject` "/Game/SupplyCo/Blueprints/BP_CommandChangeGold.BP_CommandChangeGold_C" self (* (`.Price_11_87D75CD5441D943E04940E99A4C19D17` (break `/Game/SupplyCo/Blueprints/F_ItemData` (`self.Item`))) -1)))
              (`/Game/SupplyCo/Blueprints/BP_Command.Execute` _returnvalue_4 _asbp_player_controller)
              (`self.K2_DestroyActor`)
              (`self.K2_DestroyActor` (`self.ItemInfo`))
              (`GameplayStatics.PlaySound2D` "/Game/SupplyCo/Assets/Sounds/A_CashRegister.A_CashRegister" 1.0 1.0 0.0 null null)
              (`/Game/SupplyCo/Blueprints/BP_CustomerActor.CustomerHandled` (`/Game/SupplyCo/Blueprints/BP_Gamemode.CurrentCustomer` (cast `/Game/SupplyCo/Blueprints/BP_Gamemode` (`GameplayStatics.GetGameMode`) :!pure true)))
              (else
                (`/Game/SupplyCo/Blueprints/WBP_ErrorDialogue.SetErrorText` _errorbox "You don't have enough space!")
                (`/Game/SupplyCo/Blueprints/WBP_ErrorDialogue.SetBoxVisibility` _errorbox true)))))))))

(fn `UserConstructionScript`)