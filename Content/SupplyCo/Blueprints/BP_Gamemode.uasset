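; Game mode that runs the day loop of a shop game where customers arrive one at a time to buy, sell or trigger an event.
; Each day it builds shuffled customer lists from DT_CustomerCards and queues hidden buyers and sellers scaled by Reputation, plus one factory-generated event customer.
; Speech-bubble dialogue starts each interaction, and handled-customer callbacks advance the queue.
; An empty queue shows the debt screen, with debt rising every fifth day.
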(event `self.ReceiveBeginPlay`
  (bind _asbp_player_controller (cast `/Game/SupplyCo/Blueprints/BP_PlayerController` (`GameplayStatics.GetPlayerController` 0) :!pure true))
  ;[1 1 1] Create the debug window and event factory, begin calling setup events and start the day
  (bind _returnvalue (`|CreateWidget` "/Game/SupplyCo/Blueprints/WBP_Debug.WBP_Debug_C" _asbp_player_controller))
  (`UserWidget.AddToViewport` _returnvalue 0)
  (add `/Game/SupplyCo/Blueprints/BP_PlayerController.OnDebugKeyPressed` _asbp_player_controller (delegate `DisplayDebug`))
  (`self.CreateEventFactory`)
  (`self.EnterDay`)
  (`self.Create Debt Screen`)
  (`self.Create Error Box`)
  (`self.CreateSoundSlider`))

(event `DisplayDebug`
  ;[1 1 1] Create the debug window and event factory, begin calling setup events and start the day
  (`Widget.SetVisibility` (stale `self.ReceiveBeginPlay` _returnvalue) "Visible")
  (`Widget.SetIsEnabled` (stale `self.ReceiveBeginPlay` _returnvalue) true))

(event `EnterDay`
  ;[1 1 1] Begin the day, generate customer lists and customers and show the first customer
  (`self.ClearData`)
  (`self.GenerateCustomerList` "NewEnumerator0")
  (`self.GenerateCustomerList` "NewEnumerator1")
  (`self.GenerateCustomerList` "NewEnumerator2")
  (`self.GenerateCustomers`)
  (`self.OnDayStart`)
  (`self.DisplayOneCustomer`))

(event `GenerateCustomers`
  ;[1 1 1] Create customer actors and add them to the queue
  (for _ (range (+ (/ (`/Game/SupplyCo/Blueprints/BP_PlayerController.Reputation` (cast `/Game/SupplyCo/Blueprints/BP_PlayerController` (`GameplayStatics.GetPlayerController` 0) :!pure true)) 2) 1))
    (bind _output_get (set `self.CurrentCustomerStruct` (`|GetArrayItem` (`self.BuyingCustomersList`))))
    (bind _returnvalue (`|SpawnActorFromClass` "/Game/SupplyCo/Blueprints/BP_CustomerActorBuying.BP_CustomerActorBuying_C" (`KismetMathLibrary.MakeTransform` (0.0 0.0 0.0)) "Undefined" "OverrideRootScale" null _output_get null))
    (`KismetArrayLibrary.Array_RemoveItem` (`self.BuyingCustomersList`) (`self.CurrentCustomerStruct`))
    (bind _outputcustomer (`self.SetupCustomer` _returnvalue))
    (set `self.CurrentCustomer` _outputcustomer)
    (add `/Game/SupplyCo/Blueprints/BP_CustomerActor.CustomerHandled` (`self.CurrentCustomer`) (delegate `Handle Customer Dealt With`) :!label _label))
  (for _ (range (+ (/ (`/Game/SupplyCo/Blueprints/BP_PlayerController.Reputation` (cast `/Game/SupplyCo/Blueprints/BP_PlayerController` (`GameplayStatics.GetPlayerController` 0) :!pure true)) 2) 1))
    (bind _output_get_2 (set `self.CurrentCustomerStruct` (`|GetArrayItem` (`self.SellingCustomersList`))))
    (bind _returnvalue_2 (`|SpawnActorFromClass` "/Game/SupplyCo/Blueprints/BP_CustomerActorSelling.BP_CustomerActorSelling_C" (`KismetMathLibrary.MakeTransform` (0.0 0.0 0.0)) "Undefined" "OverrideRootScale" null _output_get_2 null))
    (`KismetArrayLibrary.Array_RemoveItem` (`self.SellingCustomersList`) (`self.CurrentCustomerStruct`))
    (bind _outputcustomer_2 (`self.SetupCustomer` _returnvalue_2))
    (set `self.CurrentCustomer` _outputcustomer_2)
    (goto _label))
  (`KismetArrayLibrary.Array_Shuffle` (`self.CustomerQueue`))
  (bind _randomevent (`/Game/SupplyCo/Blueprints/BP_EventFactory.GetRandomEvent` (`self.EventFactoryRef`)))
  (bind _returnvalue_3 (`|SpawnActorFromClass` "/Game/SupplyCo/Blueprints/BP_CustomerActorEvent.BP_CustomerActorEvent_C" (`KismetMathLibrary.MakeTransform` (0.0 0.0 0.0)) "Undefined" "OverrideRootScale" null _randomevent (`|GetArrayItem` (`self.EventCustomersList`)) null))
  (bind _outputcustomer_3 (`self.SetupCustomer` _returnvalue_3))
  (set `self.CurrentCustomer` _outputcustomer_3)
  (goto _label))

(event `Handle Customer Dealt With`
  ;[1 1 1] If CustomerQueue.Size == 0 then switch state to end day
  (bind _asbp_customer_actor_buying (cast `/Game/SupplyCo/Blueprints/BP_CustomerActorBuying` (`self.ActiveCustomer`))
    (:`then`
      (bind _bubble (`/Game/SupplyCo/Blueprints/BP_CustomerActorBuying.Bubble` _asbp_customer_actor_buying)
        (:`then`
          (`self.K2_DestroyActor` (`self.GetAttachedActors` _bubble false)))
        (:`else`
          _)))
    (:`CastFailed`
      _))
  (bind _outactors (`GameplayStatics.GetAllActorsOfClass` "/Game/SupplyCo/Blueprints/BP_Bubble.BP_Bubble_C"))
  (for _array_element _outactors
    (`self.K2_DestroyActor` _array_element))
  (`self.K2_DestroyActor` (`self.ActiveCustomer`))
  (if (== (`KismetArrayLibrary.Array_Length` (`self.CustomerQueue`)) 0)
    (`self.ChangeState` "NewEnumerator1")
    (else
      (`self.ChangeState` "NewEnumerator0")
      (`self.DisplayOneCustomer`))))

(event `DisplayOneCustomer`
  ;[1 1 1] Pop a customer from the queue and display them on the screen, start their dialogue
  (bind _customeractor (`self.QueuePop` (`self.CustomerQueue`)))
  (bind _output_get (set `self.ActiveCustomer` _customeractor))
  (`self.SetActorHiddenInGame` _output_get false)
  (`self.K2_SetActorLocation` _customeractor (285.0 650.0 23.0) false false)
  (bind (_speechbubbleactor _speechbubblewidget) (`self.CreateSpeechBubble` _customeractor))
  (set `self.CurrentSpeechBubble` _speechbubbleactor)
  (add `/Game/SupplyCo/Blueprints/WBP_SpeechBubble.OnDialogueEnd` _speechbubblewidget (delegate `Start Customer Interaction`)))

(event `Start Customer Interaction`
  ;[1 1 1] Pop a customer from the queue and display them on the screen, start their dialogue
  (`/Game/SupplyCo/Blueprints/BP_CustomerActor.StartInteraction` (stale `DisplayOneCustomer` _customeractor)))

(event `CreateBackground`
  ;[1 1 1] Create background actor and add to map
  (`|SpawnActorFromClass` "/Game/SupplyCo/Blueprints/BP_BackgroundActor.BP_BackgroundActor_C" (`KismetMathLibrary.MakeTransform` (0.0 0.0 21.0)) "Undefined" "OverrideRootScale" null null))

(event `CreateEventFactory`
  ;[1 1 1] Create a list of all events and set local variable
  (bind _returnvalue (`|GenericCreateObject` "/Game/SupplyCo/Blueprints/BP_EventFactory.BP_EventFactory_C" self))
  (bind _output_get (set `self.EventFactoryRef` _returnvalue))
  (`/Game/SupplyCo/Blueprints/BP_EventFactory.CreateEvents` _output_get))

(event `Create Debt Screen`
  ;[1 1 1] Create the debt screen and display when the day is over
  (bind _returnvalue (`|CreateWidget` "/Game/SupplyCo/Blueprints/WBP_DebtScreen.WBP_DebtScreen_C" (cast `/Game/SupplyCo/Blueprints/BP_PlayerController` (`GameplayStatics.GetPlayerController` 0) :!pure true)))
  (bind _returnvalue_2 (`|SpawnActorFromClass` "/Game/SupplyCo/Blueprints/BP_DebtScreen.BP_DebtScreen_C" (`KismetMathLibrary.MakeTransform` (0.0 0.0 -100.0)) "Undefined" "OverrideRootScale" null _returnvalue null))
  (bind _asbp_hand (cast `/Game/SupplyCo/Blueprints/BP_Hand` (`ChildActorComponent.ChildActor` (`/Game/SupplyCo/Blueprints/BP_DebtScreen.Hand` _returnvalue_2))))
  (bind _output_get (set `self.Hand` _asbp_hand))
  (set `/Game/SupplyCo/Blueprints/WBP_DebtScreen.Hand` _output_get _returnvalue)
  (add `/Game/SupplyCo/Blueprints/WBP_DebtScreen.OnDayEndClicked` _returnvalue (delegate `End Day`))
  (set `self.DebtScreen` _returnvalue_2))

(event `End Day`
  ;[1 1 1] Create the debt screen and display when the day is over
  (`/Game/SupplyCo/Blueprints/BP_DebtScreen.Hide` (`self.DebtScreen`))
  (`GameplayStatics.PlaySound2D` "/Game/SupplyCo/Assets/Sounds/A_DoorBell1.A_DoorBell1" 1.0 1.0 0.0 null null)
  (`MovieSceneSequencePlayer.Play` (`LevelSequenceActor.SequencePlayer` (`self.LevelSequence`)))
  (`self.EnterDay`))

(event `Create Error Box`
  ;[1 1 1] Create error box
  (bind _returnvalue (`|CreateWidget` "/Game/SupplyCo/Blueprints/WBP_ErrorDialogue.WBP_ErrorDialogue_C" (cast `/Game/SupplyCo/Blueprints/BP_PlayerController` (`GameplayStatics.GetPlayerController` 0) :!pure true)))
  (bind _output_get (set `self.ErrorBox` _returnvalue))
  (`/Game/SupplyCo/Blueprints/WBP_ErrorDialogue.SetBoxVisibility` _output_get false)
  (`UserWidget.AddToViewport` _output_get 0))

(event `CreateSoundSlider`
  ;[1 1 1] Setup volume slider
  (bind _returnvalue (`|CreateWidget` "/Game/SupplyCo/Blueprints/WBP_VolumeAdjust.WBP_VolumeAdjust_C" (cast `/Game/SupplyCo/Blueprints/BP_PlayerController` (`GameplayStatics.GetPlayerController` 0) :!pure true)))
  (`UserWidget.AddToViewport` _returnvalue 0))

(fn `ChangeState`
  (params (NewState :type "/Game/SupplyCo/Blueprints/EGameState Enum" :default "NewEnumerator0"))
  (bind _asbp_player_controller (cast `/Game/SupplyCo/Blueprints/BP_PlayerController` (`GameplayStatics.GetPlayerController` 0) :!pure true))
  ;[1 1 1] Handle leaving old state
  (switch `/Game/SupplyCo/Blueprints/EGameState` (`self.State`)
    (:`NewEnumerator0`
      _)
    (:`NewEnumerator1`
      _)
    (:`NewEnumerator2`
      _)
    (:`NewEnumerator3`
      _)
    (:`NewEnumerator4`
      _))
  (bind _output_get (set `self.State` NewState))
  ;[1 1 1] Handle entering new state
  (switch `/Game/SupplyCo/Blueprints/EGameState` _output_get
    (:`NewEnumerator1`
      (if (== (`self.Day`) (`self.MaxDay`))
        (set `self.Day` 0)
        (else
          (bind _result (`/Engine/EditorBlueprintResources/StandardMacros.IncrementInt` (`self.Day`))
            (:`  `
              (bind _output_get_2 (set `self.Day` _result))))))
      (if (== (mod _output_get_2 5) 0)
        (`/Game/SupplyCo/Blueprints/BP_PlayerController.ChangeDebt` _asbp_player_controller (+ (`/Game/SupplyCo/Blueprints/BP_PlayerController.Debt` _asbp_player_controller) 100)))
      (`/Game/SupplyCo/Blueprints/BP_DebtScreen.Show` (`self.DebtScreen`)))))

(fn `ClearData`
  (`KismetArrayLibrary.Array_Clear` (`self.CustomerQueue`))
  (`KismetArrayLibrary.Array_Clear` (`self.SellingCustomersList`))
  (`KismetArrayLibrary.Array_Clear` (`self.EventCustomersList`))
  (`KismetArrayLibrary.Array_Clear` (`self.BuyingCustomersList`)))

(fn `CreateEventBubbleActor`
  (params (Event :type "/Game/SupplyCo/Blueprints/BP_Event Object Reference"))
  (returns (EventBubble :type "/Game/SupplyCo/Blueprints/BP_EventBubbleActor Object Reference"))
  (locals (CustomerActor :type "/Game/SupplyCo/Blueprints/BP_CustomerActor Object Reference"))
  (bind _returnvalue (`|CreateWidget` "/Game/SupplyCo/Blueprints/WBP_EventBubble.WBP_EventBubble_C" (cast `/Game/SupplyCo/Blueprints/BP_PlayerController` (`GameplayStatics.GetPlayerController` 0) :!pure true) Event))
  (bind _returnvalue_2 (`|SpawnActorFromClass` "/Game/SupplyCo/Blueprints/BP_EventBubbleActor.BP_EventBubbleActor_C" (`KismetMathLibrary.MakeTransform` (0.0 0.0 0.0)) "Undefined" "OverrideRootScale" null _returnvalue null))
  (`self.SetActorHiddenInGame` _returnvalue_2 true)
  (return _returnvalue_2))

(fn `CreateSpeechBubble`
  (params (CustomerActor :type "/Game/SupplyCo/Blueprints/BP_CustomerActor Object Reference"))
  (returns (SpeechBubbleActor :type "/Game/SupplyCo/Blueprints/BP_SpeechBubbleActor Object Reference") (SpeechBubbleWidget :type "/Game/SupplyCo/Blueprints/WBP_SpeechBubble Object Reference"))
  (locals (Customer :type "/Game/SupplyCo/Blueprints/BP_CustomerActor Object Reference") (DialogueArray :type "Array of Text"))
  (bind _dialoguearray (`local.DialogueArray`))
  (bind (_name _introdialogue _interactiondialogue) (break `/Game/SupplyCo/Blueprints/FCustomer` (`/Game/SupplyCo/Blueprints/BP_CustomerActor.Customer` CustomerActor)))
  (set `local.Customer` CustomerActor)
  ;[1 1 1] Build dialogue array for easy cycling
  (`KismetArrayLibrary.Array_Add` _dialoguearray _introdialogue)
  (`KismetArrayLibrary.Array_Add` _dialoguearray _interactiondialogue)
  (bind _returnvalue (`|CreateWidget` "/Game/SupplyCo/Blueprints/WBP_SpeechBubble.WBP_SpeechBubble_C" (cast `/Game/SupplyCo/Blueprints/BP_PlayerController` (`GameplayStatics.GetPlayerController` 0) :!pure true) (`local.DialogueArray`)))
  (bind _returnvalue_2 (`|SpawnActorFromClass` "/Game/SupplyCo/Blueprints/BP_SpeechBubbleActor.BP_SpeechBubbleActor_C" (`KismetMathLibrary.MakeTransform` (`self.K2_GetActorLocation` (`local.Customer`))) "Undefined" "OverrideRootScale" null _returnvalue null))
  (`self.K2_AddActorLocalOffset` _returnvalue_2 (-50.0 -350.0 1.0) false false)
  (return _returnvalue_2 _returnvalue))

(fn `GenerateCustomerList`
  (params (CustomerType :type "/Game/SupplyCo/Blueprints/ECustomerType Enum" :default "NewEnumerator0"))
  (locals (CurrentFCustomer :type "/Game/SupplyCo/Blueprints/FCustomer Structure"))
  (switch `/Game/SupplyCo/Blueprints/ECustomerType` CustomerType
    (:`NewEnumerator0`
      (bind _outrownames (`DataTableFunctionLibrary.GetDataTableRowNames` "/Game/SupplyCo/Blueprints/DT_CustomerCards.DT_CustomerCards"))
      (for _array_element _outrownames
        (bind _returnvalue (`|GetDataTableRow` "/Game/SupplyCo/Blueprints/DT_CustomerCards.DT_CustomerCards" _array_element)
          (:`then`
            (bind _output_get (set `local.CurrentFCustomer` _returnvalue))
            (if (`|EnumEquality` (`.CustomerType_31_E07EF9F64E8F0E4F93516DA369D4952D` (break `/Game/SupplyCo/Blueprints/FCustomer` _output_get)) "NewEnumerator0")
              (`KismetArrayLibrary.Array_Add` (`self.SellingCustomersList`) (`local.CurrentFCustomer`))
              (`KismetArrayLibrary.Array_Shuffle` (`self.SellingCustomersList`)))))))
    (:`NewEnumerator1`
      (bind _outrownames_2 (`DataTableFunctionLibrary.GetDataTableRowNames` "/Game/SupplyCo/Blueprints/DT_CustomerCards.DT_CustomerCards"))
      (for _array_element_2 _outrownames_2
        (bind _returnvalue_2 (`|GetDataTableRow` "/Game/SupplyCo/Blueprints/DT_CustomerCards.DT_CustomerCards" _array_element_2)
          (:`then`
            (bind _output_get_2 (set `local.CurrentFCustomer` _returnvalue_2))
            (if (`|EnumEquality` (`.CustomerType_31_E07EF9F64E8F0E4F93516DA369D4952D` (break `/Game/SupplyCo/Blueprints/FCustomer` _output_get_2)) "NewEnumerator1")
              (`KismetArrayLibrary.Array_Add` (`self.EventCustomersList`) (`local.CurrentFCustomer`))
              (`KismetArrayLibrary.Array_Shuffle` (`self.EventCustomersList`)))))))
    (:`NewEnumerator2`
      (bind _outrownames_3 (`DataTableFunctionLibrary.GetDataTableRowNames` "/Game/SupplyCo/Blueprints/DT_CustomerCards.DT_CustomerCards"))
      (for _array_element_3 _outrownames_3
        (bind _returnvalue_3 (`|GetDataTableRow` "/Game/SupplyCo/Blueprints/DT_CustomerCards.DT_CustomerCards" _array_element_3)
          (:`then`
            (bind _output_get_3 (set `local.CurrentFCustomer` _returnvalue_3))
            (if (`|EnumEquality` (`.CustomerType_31_E07EF9F64E8F0E4F93516DA369D4952D` (break `/Game/SupplyCo/Blueprints/FCustomer` _output_get_3)) "NewEnumerator2")
              (`KismetArrayLibrary.Array_Add` (`self.BuyingCustomersList`) (`local.CurrentFCustomer`))
              (`KismetArrayLibrary.Array_Shuffle` (`self.BuyingCustomersList`)))))))))

(fn `QueuePop`
  (params (Queue :type "Array of /Game/SupplyCo/Blueprints/BP_CustomerActor Object Reference"))
  (returns (CustomerActor :type "/Game/SupplyCo/Blueprints/BP_CustomerActor Object Reference"))
  (locals (Customer :type "/Game/SupplyCo/Blueprints/BP_CustomerActor Object Reference"))
  (set `local.Customer` (`|GetArrayItem` Queue))
  (`KismetArrayLibrary.Array_Remove` Queue)
  (return (`local.Customer`)))

(fn `SetupCustomer`
  (params (Customer :type "/Game/SupplyCo/Blueprints/BP_CustomerActor Object Reference"))
  (returns (OutputCustomer :type "/Game/SupplyCo/Blueprints/BP_CustomerActor Object Reference"))
  (locals (CustomerActor :type "/Game/SupplyCo/Blueprints/BP_CustomerActor Object Reference"))
  (bind _customeractor (`local.CustomerActor`))
  (bind _output_get (set `local.CustomerActor` Customer))
  (`KismetArrayLibrary.Array_Add` (`self.CustomerQueue`) _output_get)
  (`self.SetActorHiddenInGame` _customeractor true)
  (return _customeractor))

(fn `UserConstructionScript`)