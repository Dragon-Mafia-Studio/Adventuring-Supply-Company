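; BP_DebtScreen is an actor that presents the debt screen through a widget component.
; On BeginPlay it assigns DebtScreenWidget to that component.
; Show and Hide toggle visibility on the root and its children, and also move the actor between fixed locations, raised when shown and sunk below the origin when hidden.
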(event `self.ReceiveBeginPlay`
  (`WidgetComponent.SetWidget` (`self.Widget`) (`self.DebtScreenWidget`)))

(fn `Hide`
  (`SceneComponent.SetHiddenInGame` (`self.DefaultSceneRoot`) true true)
  (`self.K2_SetActorLocation` (0.0 0.0 -100.0)))

(fn `Show`
  (`SceneComponent.SetHiddenInGame` (`self.DefaultSceneRoot`) false true)
  (`self.K2_SetActorLocation` (0.0 0.0 40.0)))

(fn `UserConstructionScript`)