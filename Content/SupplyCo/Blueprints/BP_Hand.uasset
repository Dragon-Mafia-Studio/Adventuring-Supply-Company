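; BP_Hand is a five-fingered hand actor that loses fingers as the player controller reports changes to the finger count.
; BeginPlay fills an ordered Fingers array from thumb to pinky and binds UpdateFingers to the controller's OnFingersChanged event.
; Each event destroys the first remaining finger component, ignoring the RemainingFingers value and without checking for an empty array.
; HideHand and ShowHand toggle in-game visibility through the root, propagating to children.
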(event `self.ReceiveBeginPlay`
  (set `self.Fingers` (`|MakeArray` (`self.Thumb`) (`self.Pointer`) (`self.Middle`) (`self.Ring`) (`self.Pinky`)))
  (add `/Game/SupplyCo/Blueprints/BP_PlayerController.OnFingersChanged` (cast `/Game/SupplyCo/Blueprints/BP_PlayerController` (`GameplayStatics.GetPlayerController` 0) :!pure true) (delegate `Update Fingers`)))

(event `Update Fingers`
  (params (RemainingFingers :type Integer))
  (`self.RemoveFinger`))

(fn `HideHand`
  (`SceneComponent.SetHiddenInGame` (`self.DefaultSceneRoot`) true true))

(fn `RemoveFinger`
  (bind _output (`|GetArrayItem` (`self.Fingers`)))
  (`ActorComponent.K2_DestroyComponent` _output)
  (`KismetArrayLibrary.Array_RemoveItem` (`self.Fingers`) _output))

(fn `ShowHand`
  (`SceneComponent.SetHiddenInGame` (`self.DefaultSceneRoot`) false true))

(fn `UserConstructionScript`)