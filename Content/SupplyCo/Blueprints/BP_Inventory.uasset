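; BP_Inventory is an inventory Actor that stores item data structs in a size-limited array.
; AddItem appends while below MaxSize and broadcasts an item-added event with itself as the inventory.
; RemoveItem finds the item, replaces it with a copy flagged Delete, removes flagged entries while looping over the array, then broadcasts an item-removed event using the loop's element.
; Removing a missing item only prints a message.
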(fn `AddItem`
  (params (Item :type "/Game/SupplyCo/Blueprints/F_ItemData Structure"))
  (returns (IsSuccessful :type Boolean))
  (locals (Added :type Boolean :default true))
  (if (>= (`KismetArrayLibrary.Array_Length` (`self.Items`)) (`self.MaxSize`))
    (set `local.Added` false)
    (else
      (`KismetArrayLibrary.Array_Add` (`self.Items`) Item)
      (`self.OnItemAdded` Item self)))
  (return (`local.Added`)))

(fn `RemoveItem`
  (params (Item :type "/Game/SupplyCo/Blueprints/F_ItemData Structure"))
  (bind (_name _itemdescription _price _picture _uid) (break `/Game/SupplyCo/Blueprints/F_ItemData` (`self.Item`)))
  (bind _output_get (set `self.Item` Item))
  (bind _returnvalue (`KismetArrayLibrary.Array_Find` (`self.Items`) _output_get))
  (set `self.FoundIndex` _returnvalue)
  (if (>= _returnvalue 0)
    (bind _output_get_2 (set `self.Item` (make `/Game/SupplyCo/Blueprints/F_ItemData` _name _itemdescription _price _picture _uid true)))
    (`self.ReplaceElement` (`self.FoundIndex`) _output_get_2)
    (for (_array_element _array_index) (`self.Items`)
      (if (`.Delete?_22_C0BBD168438B9B9D241348BA93701B69` (break `/Game/SupplyCo/Blueprints/F_ItemData` _array_element))
        (`KismetArrayLibrary.Array_Remove` (`self.Items`) _array_index)))
    (`self.OnItemRemoved` _array_element self)
    (else
      (`KismetSystemLibrary.PrintString` "Attempted to remove Item not in inventory"))))

(fn `ReplaceElement`
  (params (Index :type Integer) (ItemToAdd :type "/Game/SupplyCo/Blueprints/F_ItemData Structure"))
  (`KismetArrayLibrary.Array_Set` (`self.Items`) Index ItemToAdd))

(fn `UserConstructionScript`)