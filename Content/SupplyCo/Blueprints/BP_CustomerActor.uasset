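; Actor representing a customer, which signals when the player double-clicks it.
; On BeginPlay it applies the customer's image to its Paper2D sprite and fills a widget component with a nameplate showing the customer's name.
; Sprite clicks increment a counter that a 0.25-second retriggerable delay resets, and a count of two calls CustomerHandled.
; StartInteraction and the construction script are empty.
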(event `self.ReceiveBeginPlay`
  (bind (_name _introdialogue _interactiondialogue _image) (break `/Game/SupplyCo/Blueprints/FCustomer` (`self.Customer`)))
  ;[1 1 1] Set name, description, image based on customer
  (set `self.Name` _name)
  (`PaperSpriteComponent.SetSprite` (`self.PaperSprite`) _image)
  (bind _returnvalue (`|CreateWidget` "/Game/SupplyCo/Blueprints/WBP_Nameplate.WBP_Nameplate_C" (cast `/Game/SupplyCo/Blueprints/BP_PlayerController` (`GameplayStatics.GetPlayerController` 0) :!pure true) (`self.Name`)))
  (`WidgetComponent.SetWidget` (`self.Widget`) _returnvalue))

(event `self.PaperSprite.OnClicked`
  (params (TouchedComponent :type "PrimitiveComponent Object Reference") (ButtonPressed :type "Key Structure"))
  (`self.Handle Click`))

(event `Handle Click`
  (`|ExecutionSequence`
    (:`then_0`
      (set `self.ClickAmount` (+ (`self.ClickAmount`) 1))
      (`KismetSystemLibrary.RetriggerableDelay` 0.25)
      (set `self.ClickAmount` 0))
    (:`then_1`
      (if (== (`self.ClickAmount`) 2)
        (`self.CustomerHandled`)))))

(fn `StartInteraction`)

(fn `UserConstructionScript`)