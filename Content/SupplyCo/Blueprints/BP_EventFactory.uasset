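; BP_EventFactory builds and serves the shop's narrative events, such as a refund request or a brawl outside, each offering the player a choice.
; CreateEvents hard-codes each BP_Event with named FEventOption choices and appends it to EventArray.
; Each option carries constructed command objects that change gold or reputation, so consequences follow a command pattern.
; GetEventByIndex looks up the array, and GetRandomEvent uses it to pick one at random.
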(fn `CreateEvents`
  (returns (EventArray :type "Array of /Game/SupplyCo/Blueprints/BP_Event Object Reference"))
  ;[1 1 1] Stolen Sword
  (bind _returnvalue (`|GenericCreateObject` "/Game/SupplyCo/Blueprints/BP_CommandChangeReputation.BP_CommandChangeReputation_C" self 1))
  (bind _returnvalue_2 (`|GenericCreateObject` "/Game/SupplyCo/Blueprints/BP_CommandChangeGold.BP_CommandChangeGold_C" self -100))
  (bind _returnvalue_3 (`|GenericCreateObject` "/Game/SupplyCo/Blueprints/BP_CommandChangeReputation.BP_CommandChangeReputation_C" "/Game/SupplyCo/Blueprints/BP_Command.BP_Command" -1))
  (bind _returnvalue_4 (`|GenericCreateObject` "/Game/SupplyCo/Blueprints/BP_CommandChangeGold.BP_CommandChangeGold_C" self 100))
  (bind _returnvalue_5 (`|GenericCreateObject` "/Game/SupplyCo/Blueprints/BP_Event.BP_Event_C" self (`|MakeArray` (make `/Game/SupplyCo/Blueprints/FEventOption` "New Weapon" (`|MakeArray` _returnvalue _returnvalue_2 :!type "/Game/SupplyCo/Blueprints/BP_Command Object Reference")) (make `/Game/SupplyCo/Blueprints/FEventOption` "Charge Them" (`|MakeArray` _returnvalue_4 _returnvalue_3 :!type "/Game/SupplyCo/Blueprints/BP_Command Object Reference"))) "Stolen Sword" "\"You sold me a sword last week, but some little ruffian stole it. Can you give me a refund?\""))
  (`KismetArrayLibrary.Array_Add` (`self.EventArray`) _returnvalue_5)
  ;[1 1 1] Shop Brawl
  (bind _returnvalue_6 (`|GenericCreateObject` "/Game/SupplyCo/Blueprints/BP_CommandChangeReputation.BP_CommandChangeReputation_C" self 1))
  (bind _returnvalue_7 (`|GenericCreateObject` "/Game/SupplyCo/Blueprints/BP_CommandChangeReputation.BP_CommandChangeReputation_C" "/Game/SupplyCo/Blueprints/BP_Command.BP_Command" -1))
  (bind _returnvalue_8 (`|GenericCreateObject` "/Game/SupplyCo/Blueprints/BP_Event.BP_Event_C" self (`|MakeArray` (make `/Game/SupplyCo/Blueprints/FEventOption` "Break it up" (`|MakeArray` _returnvalue_6 :!type "/Game/SupplyCo/Blueprints/BP_Command Object Reference")) (make `/Game/SupplyCo/Blueprints/FEventOption` "Ignore It" (`|MakeArray` _returnvalue_7 :!type "/Game/SupplyCo/Blueprints/BP_Command Object Reference"))) "Shop Brawl" "A fight broke out in front of your shop and the situation could be simply ended if a certain shop owner intimidated the ruffians with a weapon . Will you go help?"))
  (`KismetArrayLibrary.Array_Add` (`self.EventArray`) _returnvalue_8)
  ;[1 1 1] A "Friend"
  (bind _returnvalue_9 (`|GenericCreateObject` "/Game/SupplyCo/Blueprints/BP_CommandChangeReputation.BP_CommandChangeReputation_C" self 2))
  (bind _returnvalue_10 (`|GenericCreateObject` "/Game/SupplyCo/Blueprints/BP_CommandChangeGold.BP_CommandChangeGold_C" self -200))
  (bind _returnvalue_11 (`|GenericCreateObject` "/Game/SupplyCo/Blueprints/BP_CommandChangeReputation.BP_CommandChangeReputation_C" self -1))
  (bind _returnvalue_12 (`|GenericCreateObject` "/Game/SupplyCo/Blueprints/BP_Event.BP_Event_C" self (`|MakeArray` (make `/Game/SupplyCo/Blueprints/FEventOption` "... Sure Pal" (`|MakeArray` _returnvalue_10 _returnvalue_9 :!type "/Game/SupplyCo/Blueprints/BP_Command Object Reference")) (make `/Game/SupplyCo/Blueprints/FEventOption` "Nah." (`|MakeArray` _returnvalue_11))) "A \"Friend\"" "I'm what you would call a 'friend' of your pals in the Dragon Mafia cuz I like to keep my enemies close, ya know? If you give me some coin, I'd make sure no one in town hears that those scaly creeps that fund your shop."))
  (`KismetArrayLibrary.Array_Add` (`self.EventArray`) _returnvalue_12)
  ;[1 1 1] The Curse
  (bind _returnvalue_13 (`|GenericCreateObject` "/Game/SupplyCo/Blueprints/BP_CommandChangeReputation.BP_CommandChangeReputation_C" self -3))
  (bind _returnvalue_14 (`|GenericCreateObject` "/Game/SupplyCo/Blueprints/BP_CommandChangeGold.BP_CommandChangeGold_C" self 400))
  (bind _returnvalue_15 (`|GenericCreateObject` "/Game/SupplyCo/Blueprints/BP_CommandChangeReputation.BP_CommandChangeReputation_C" self 2))
  (bind _returnvalue_16 (`|GenericCreateObject` "/Game/SupplyCo/Blueprints/BP_Event.BP_Event_C" self (`|MakeArray` (make `/Game/SupplyCo/Blueprints/FEventOption` "Sure!" (`|MakeArray` _returnvalue_14 _returnvalue_13 :!type "/Game/SupplyCo/Blueprints/BP_Command Object Reference")) (make `/Game/SupplyCo/Blueprints/FEventOption` "Go away!" (`|MakeArray` _returnvalue_15))) "The Curse" "So, I may or may not have been cursed by a sea demon, and I was wondering if you would help me to get rid of it? I figured that you'd have a wand that could help, but this may take a while… and may cost you a customer or two."))
  (`KismetArrayLibrary.Array_Add` (`self.EventArray`) _returnvalue_16)
  (return (`self.EventArray`)))

(fn `GetEventByIndex`
  (params (Index :type Integer))
  (returns (Event :type "/Game/SupplyCo/Blueprints/BP_Event Object Reference"))
  (return (`|GetArrayItem` (`self.EventArray`) Index)))

(fn `GetRandomEvent`
  (returns (RandomEvent :type "/Game/SupplyCo/Blueprints/BP_Event Object Reference"))
  (bind _event (`self.GetEventByIndex` (`KismetMathLibrary.RandomInteger` (`KismetArrayLibrary.Array_Length` (`self.EventArray`)))))
  (return _event))