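; BP_Shelf is a shelf actor that displays inventory items as physical item actors in slots.
; On BeginPlay it waits for the player controller to create its inventory, then listens for added items.
; Each added item spawns a BP_ItemActor flagged as in inventory, placed into the first free slot.
; When every slot is taken, it only prints an error, with no guard on the empty result.
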(event `self.ReceiveBeginPlay`
  (bind _asbp_player_controller (cast `/Game/SupplyCo/Blueprints/BP_PlayerController` (`GameplayStatics.GetPlayerController` 0)))
  (add `/Game/SupplyCo/Blueprints/BP_PlayerController.OnInventoryCreated` _asbp_player_controller (delegate `ListenForItems`)))

(event `ListenForItems`
  (params (Inventory :type "/Game/SupplyCo/Blueprints/BP_Inventory Object Reference"))
  (add `/Game/SupplyCo/Blueprints/BP_Inventory.OnItemAdded` Inventory (delegate `OnItemAdded`)))

(event `OnItemAdded`
  (params (ItemAdded :type "/Game/SupplyCo/Blueprints/F_ItemData Structure") (Inventory :type "/Game/SupplyCo/Blueprints/BP_Inventory Object Reference"))
  (bind _returnvalue (`|SpawnActorFromClass` "/Game/SupplyCo/Blueprints/BP_ItemActor.BP_ItemActor_C" (`KismetMathLibrary.MakeTransform` (0.0 0.0 0.0)) "Undefined" "OverrideRootScale" null ItemAdded null))
  (set `/Game/SupplyCo/Blueprints/BP_ItemActor.IsInInventory` true _returnvalue)
  (`self.AddItem` _returnvalue))

(fn `AddItem`
  (params (Item :type "/Game/SupplyCo/Blueprints/BP_ItemActor Object Reference"))
  (bind _availableslot (`self.GetEmptySlot`))
  (`/Game/SupplyCo/Blueprints/BP_ShelfSlot.AddItemToSlot` _availableslot Item))

(fn `GetEmptySlot`
  (returns (AvailableSlot :type "/Game/SupplyCo/Blueprints/BP_ShelfSlot Object Reference"))
  (for _array_element (`self.Slots`)
    (if (not (`/Game/SupplyCo/Blueprints/BP_ShelfSlot.IsTaken` _array_element))
      (return _array_element)))
  (`KismetSystemLibrary.PrintString` "ERROR. INVENTORY FULL"))

(fn `UserConstructionScript`)