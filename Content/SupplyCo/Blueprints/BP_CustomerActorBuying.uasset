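; Customer actor for a buying interaction, which shows a random item card in a speech bubble.
; StartInteraction changes the gamemode state and spawns a bubble actor wrapping a buying widget, offset from the customer and filled with a random DT_ItemCards row.
; It listens for the player controller's inventory creation, then for added items; an addition during that state destroys the bubble and signals the customer as handled.
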(event `self.ReceiveBeginPlay`
  (`parent.ReceiveBeginPlay`)
  (add `/Game/SupplyCo/Blueprints/BP_PlayerController.OnInventoryCreated` (cast `/Game/SupplyCo/Blueprints/BP_PlayerController` (`GameplayStatics.GetPlayerController` 0) :!pure true) (delegate `OnInventoryCreated`)))

(event `OnInventoryCreated`
  (params (Inventory :type "/Game/SupplyCo/Blueprints/BP_Inventory Object Reference"))
  (add `/Game/SupplyCo/Blueprints/BP_Inventory.OnItemAdded` Inventory (delegate `Handle Customer`)))

(event `Handle Customer`
  (params (ItemAdded :type "/Game/SupplyCo/Blueprints/F_ItemData Structure") (Inventory :type "/Game/SupplyCo/Blueprints/BP_Inventory Object Reference"))
  (if (`|EnumEquality` (`/Game/SupplyCo/Blueprints/BP_Gamemode.State` (cast `/Game/SupplyCo/Blueprints/BP_Gamemode` (`GameplayStatics.GetGameMode`) :!pure true)) "NewEnumerator3")
    (bind _bubble (`self.Bubble`)
      (:`then`
        (`self.K2_DestroyActor` _bubble))
      (:`else`
        _))
    (`self.CustomerHandled`)))

(fn `CreateBuyingBubble`
  (returns (BubbleActor :type "/Game/SupplyCo/Blueprints/BP_BuyingBubbleActor Object Reference"))
  (bind _returnvalue (`|CreateWidget` "/Game/SupplyCo/Blueprints/WBP_BuyingBubble.WBP_BuyingBubble_C" (cast `/Game/SupplyCo/Blueprints/BP_PlayerController` (`GameplayStatics.GetPlayerController` 0) :!pure true)))
  (bind _returnvalue_2 (`|SpawnActorFromClass` "/Game/SupplyCo/Blueprints/BP_BuyingBubbleActor.BP_BuyingBubbleActor_C" (`KismetMathLibrary.MakeTransform` (0.0 0.0 0.0)) "Undefined" "OverrideRootScale" null _returnvalue null))
  (bind _output_get (set `self.Bubble` _returnvalue_2))
  (`self.K2_SetActorLocation` _output_get (`self.K2_GetActorLocation` self) false false)
  (`self.K2_AddActorLocalOffset` _output_get (-50.0 -350.0 1.0) false false)
  (bind _outrownames (`DataTableFunctionLibrary.GetDataTableRowNames` "/Game/SupplyCo/Blueprints/DT_ItemCards.DT_ItemCards"))
  (bind _returnvalue_3 (`|GetDataTableRow` "/Game/SupplyCo/Blueprints/DT_ItemCards.DT_ItemCards" (`|GetArrayItem` _outrownames (`KismetMathLibrary.RandomInteger` (`KismetArrayLibrary.Array_Length` _outrownames))))
    (:`then`
      (`/Game/SupplyCo/Blueprints/BP_BuyingBubbleActor.AddItem` _output_get _returnvalue_3)
      (return (`self.Bubble`)))))

(fn `StartInteraction`
  (`/Game/SupplyCo/Blueprints/BP_Gamemode.ChangeState` (cast `/Game/SupplyCo/Blueprints/BP_Gamemode` (`GameplayStatics.GetGameMode`) :!pure true) "NewEnumerator3")
  (`self.CreateBuyingBubble`))

(fn `UserConstructionScript`)